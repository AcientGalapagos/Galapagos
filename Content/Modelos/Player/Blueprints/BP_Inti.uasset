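; BP_Inti is the third-person player character, with movement, sprint, montage-driven jump, a two-camera zoom toggle and stone firing.
; Hits while the grab input is held attach crates to a PhysicsHandle, updated every tick until dropped or impulse-thrown.
; Damage reduces health; death saves the current transform as respawn point, requests game mode regeneration and destroys the actor.
; It also tracks a key, stones, kills and animal rescues, forwarding score to the game mode.
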(event `self.ReceiveBeginPlay`
  ;[1 1 1] BEGIN PLAY
  (`|ExecutionSequence`
    (:`then_0`
      (`self.LIMITESCAMARA`))
    (:`then_1`
      (`self.RESETVARIABLES`))
    (:`then_2`
      (`self.ACTUALIZAPUNTOGENERACION`))))

(event `self.ReceiveTick`
  (params (DeltaSeconds :type "Float (single-precision)"))
  ;[1 1 1] EVENTO TICK
  (`|ExecutionSequence`
    (:`then_0`
      (`self.NUEVAPOSICIONCAJA`))))

(event `ACTUALIZAPUNTOGENERACION`
  ;[1 1 1] PUNTO DE regeneracion del personaje
  (bind _asbp_gm_tercera_persona (cast `/Game/Modelos/Player/Blueprints/BP_GM_terceraPersona` (`GameplayStatics.GetGameMode`)))
  (bind _output_get (set `self.MODODEJUEGO` _asbp_gm_tercera_persona))
  (set `/Game/Modelos/Player/Blueprints/BP_GM_terceraPersona.PUNTOGEGENERACION` (`self.GetTransform`) _output_get))

(event `AgarrarLlave`
  ;[1 1 1] CONTROL LLAVE
  (set `self.llave` true))

(event `RESETVARIABLES`
  ;[1 1 1] RESET VARIABLES
  (`|ExecutionSequence`
    (:`then_0`
      (set `self.ESTASVIVO` true))
    (:`then_1`
      (set `self.VIDA` 100))))

(event `tieneLlave`
  ;[1 1 1] CONTROL LLAVE
  (if (`self.llave`)
    (`KismetSystemLibrary.PrintString` "Abre la puerta")
    (else
      (`KismetSystemLibrary.PrintString` "Te falta una llave"))))

(event `LIMITESCAMARA`
  (bind _returnvalue (`GameplayStatics.GetPlayerCameraManager` 0))
  ;[1 1 1] CONTROL CAMARA
  ;;[1 1 1] LIMITES
  (set `PlayerCameraManager.ViewPitchMax` 40.0 _returnvalue)
  (set `PlayerCameraManager.ViewPitchMin` -20.0 _returnvalue))

(event `InputAxis|Turn`
  (params (AxisValue :type "Float (single-precision)"))
  ;[1 1 1] CONTROL CAMARA
  ;;[1 1 1] MOVIMIENTO
  (`self.AddControllerYawInput` AxisValue))

(event `InputAxis|LookUp`
  (params (AxisValue :type "Float (single-precision)"))
  ;[1 1 1] CONTROL CAMARA
  ;;[1 1 1] MOVIMIENTO
  (`self.AddControllerPitchInput` AxisValue))

(event `REDUCIRVIDA`
  (params (`DAÑO` :type Integer))
  ;[1 1 1] REDUCIR VIDA EN UN ATAQUE
  (if (`self.ESTASVIVO`)
    (bind _output_get (set `self.VIDA` (- (`self.VIDA`) `DAÑO`)))
    (if (<= _output_get 0)
      (set `self.ESTASVIVO` false)
      (`self.ACTUALIZAPUNTOGENERACION`)
      (else
        (set `self.ESTASVIVO` true)))))

(event `InputAction|zoom`
  (params (Key :type "Key Structure"))
  ;[1 1 1] CAMBIO CAMARA - ZOOM
  (:`Pressed`
    (`/Engine/EditorBlueprintResources/StandardMacros.FlipFlop`
      (:`A`
        (`ActorComponent.Deactivate` (`self.playerCam`))
        (`ActorComponent.Activate` (`self.tercerCam`) false))
      (:`B`
        (`ActorComponent.Deactivate` (`self.tercerCam`))
        (`ActorComponent.Activate` (`self.playerCam`) false)))))

(event `InputAction|lanzar`
  (params (Key :type "Key Structure"))
  ;[1 1 1] LANZAR OBJETOS
  (:`Pressed`
    (if (`self.TENGOOBJETO`)
      (`PhysicsHandleComponent.ReleaseComponent` (`self.PhysicsHandle`))
      (`PrimitiveComponent.AddImpulse` (`self.COMPONENTECAJA`) (* (`self.GetActorForwardVector`) 1000) "None" true)
      (set `self.COMPONENTECAJA` null)
      (`CharacterMovementComponent.AddImpulse` (`self.CharacterMovement`) (* (`KismetMathLibrary.GetForwardVector` (struct)) -5000) true)
      (set `self.TENGOOBJETO` false))))

(event `InputAxis|MoveForward`
  (params (AxisValue :type "Float (single-precision)"))
  ;[1 1 1] MOVIMIENTO PLAYER
  (`self.AddMovementInput` (`KismetMathLibrary.GetForwardVector` (`KismetMathLibrary.MakeRotator` 0.0 0.0 (.yaw (`self.GetControlRotation`)))) AxisValue))

(event `InputAxis|MoveRight`
  (params (AxisValue :type "Float (single-precision)"))
  ;[1 1 1] MOVIMIENTO PLAYER
  (`self.AddMovementInput` (`KismetMathLibrary.GetRightVector` (`KismetMathLibrary.MakeRotator` 0.0 0.0 (.yaw (`self.GetControlRotation`)))) AxisValue))

(event `InputAction|COGER`
  (params (Key :type "Key Structure"))
  ;[1 1 1] COGER OBJETOS
  (:`Pressed`
    (set `self.COGEROBJETO` true))
  (:`Released`
    (set `self.COGEROBJETO` false)))

(event `InputAction|SOLTAR`
  (params (Key :type "Key Structure"))
  ;[1 1 1] SOLTAR OBJETOS
  (:`Pressed`
    (`PhysicsHandleComponent.ReleaseComponent` (`self.PhysicsHandle`))
    (set `self.TENGOOBJETO` false)))

(event `InputAction|runing`
  (params (Key :type "Key Structure"))
  (bind _charactermovement (`self.CharacterMovement`))
  ;[1 1 1] MOVIMIENTO PLAYER
  (:`Pressed`
    (if (`self.enSuelo`)
      (set `self.isRun` true)
      (set `CharacterMovementComponent.MaxWalkSpeed` 600.0 _charactermovement)))
  (:`Released`
    (if (`self.enSuelo`)
      (set `self.isRun` false)
      (set `CharacterMovementComponent.MaxWalkSpeed` 300.0 _charactermovement))))

(event `self.ReceiveHit`
  (params (MyComp :type "PrimitiveComponent Object Reference") (Other :type "Actor Object Reference") (OtherComp :type "PrimitiveComponent Object Reference") (bSelfMoved :type Boolean) (HitLocation :type "Vector Structure") (HitNormal :type "Vector Structure") (NormalImpulse :type "Vector Structure") (Hit :type "HitResult Structure (by ref)"))
  ;[1 1 1] COGER OBJETOS
  (if (`self.COGEROBJETO`)
    (if (not (`self.TENGOOBJETO`))
      (`|ExecutionSequence`
        (:`then_0`
          (cast `/Game/BpClass/CAJA1` Other))
        (:`then_1`
          (cast `/Game/BpClass/CAJA2` Other))
        (:`then_2`
          (cast `/Game/BpClass/CAJA3` Other)))
      (`PhysicsHandleComponent.GrabComponentAtLocation` (`self.PhysicsHandle`) OtherComp "None" (`SceneComponent.K2_GetComponentLocation` OtherComp))
      (set `self.COMPONENTECAJA` OtherComp)
      (set `self.TENGOOBJETO` true))))

(event `InputAction|jump`
  (params (Key :type "Key Structure"))
  ;[1 1 1] ACCION SALTAR
  (:`Pressed`
    (if (`self.enSuelo`)
      (`self.Jump`)
      (`|PlayMontage` (`self.Mesh`) "/Game/Modelos/Player/amins/AM_JumInti.AM_JumInti" 0.9
        (:`then`
          (if (`NavMovementComponent.IsFalling` (`self.CharacterMovement`))
            (set `self.enSuelo` false)
            (else
              (set `self.enSuelo` true))))))))

(event `NUEVAPOSICIONCAJA`
  ;[1 1 1] COGER OBJETOS
  (`PhysicsHandleComponent.SetTargetLocation` (`self.PhysicsHandle`) (`SceneComponent.K2_GetComponentLocation` (`self.POSICIONCAJA`))))

(event `self.OnLanded`
  (params (Hit :type "HitResult Structure (by ref)"))
  ;[1 1 1] ACCION SALTAR
  (`|PlayMontage` (`self.Mesh`) "/Game/Modelos/Player/amins/AM_JumInti.AM_JumInti" 1.0 0.0 "CaidaEnd"
    (:`then`
      (set `self.enSuelo` true))))

(event `InputAction|disparar`
  (params (Key :type "Key Structure"))
  ;[1 1 1] DISPARAR
  (:`Pressed`
    (`|SpawnActorFromClass` "/Game/BpClass/PIEDRA.PIEDRA_C" (`SceneComponent.K2_GetComponentToWorld` (`self.POSICIONARMA`)) "Undefined" "OverrideRootScale" null null)))

(event `IMPACTO`
  (params (`DAÑO` :type Integer))
  ;[1 1 1] IMPACTO EN JUGADOR PRINCIPAL
  (`self.REDUCIRVIDA` `DAÑO`)
  (if (> (`self.VIDA`) 0)
    (`KismetSystemLibrary.PrintString` (`KismetStringLibrary.Concat_StrStr` "VIDA ACTUAL: " (`KismetStringLibrary.Conv_IntToString` (`self.VIDA`))))
    (else
      (`KismetSystemLibrary.PrintString` "EL JUGADOR ESTA MUERTO")
      (`/Game/Modelos/Player/Blueprints/BP_GM_terceraPersona.REGENERARJUGADOR` (`self.MODODEJUEGO`))
      (`self.K2_DestroyActor` self))))

(event `SUMAPUNTOS`
  (params (PUNTOS :type "Float (double-precision)"))
  (bind _mododejuego (`self.MODODEJUEGO`))
  ;[1 1 1] INCREMENTO DE SCORING
  (set `/Game/Modelos/Player/Blueprints/BP_GM_terceraPersona.PUNTUACION` (+ PUNTOS (`/Game/Modelos/Player/Blueprints/BP_GM_terceraPersona.PUNTUACION` _mododejuego)) _mododejuego))

(event `IncContadorEnemigos`
  ;[1 1 1] INCREMENTO DE CONTADORES PARCIALES
  (bind _result (`/Engine/EditorBlueprintResources/StandardMacros.IncrementFloat` (`self.ENEMIGOSMUERTOS`))
    (:`  `
      (set `self.ENEMIGOSMUERTOS` _result))))

(event `IncContadorTortugas`
  ;[1 1 1] INCREMENTO DE CONTADORES PARCIALES
  (bind _result (`/Engine/EditorBlueprintResources/StandardMacros.IncrementFloat` (`self.TORTUGASRESCATADAS`))
    (:`  `
      (set `self.TORTUGASRESCATADAS` _result))))

(event `IncContadorLeones`
  ;[1 1 1] INCREMENTO DE CONTADORES PARCIALES
  (bind _result (`/Engine/EditorBlueprintResources/StandardMacros.IncrementFloat` (`self.LEONESRESCATADOS`))
    (:`  `
      (set `self.LEONESRESCATADOS` _result))))

(event `IncContadorIguanas`
  ;[1 1 1] INCREMENTO DE CONTADORES PARCIALES
  (bind _result (`/Engine/EditorBlueprintResources/StandardMacros.IncrementFloat` (`self.IGUANASRESCATADAS`))
    (:`  `
      (set `self.IGUANASRESCATADAS` _result))))

(event `IncContadorPiedras`
  ;[1 1 1] INCREMENTO DE CONTADORES PARCIALES
  ;;[1 1 1] CONTADORES DE PIEDRAS COMO PROYECTILES
  (bind _result (`/Engine/EditorBlueprintResources/StandardMacros.IncrementInt` (`self.PIEDRAS`))
    (:`  `
      (set `self.PIEDRAS` _result))))

(event `DecContadorPiedras`
  ;[1 1 1] INCREMENTO DE CONTADORES PARCIALES
  ;;[1 1 1] CONTADORES DE PIEDRAS COMO PROYECTILES
  (bind _result (`/Engine/EditorBlueprintResources/StandardMacros.DecrementInt` (`self.PIEDRAS`))
    (:`  `
      (set `self.PIEDRAS` _result))))

(fn `UserConstructionScript`)