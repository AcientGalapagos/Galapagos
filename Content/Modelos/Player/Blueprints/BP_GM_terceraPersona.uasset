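; Third-person game mode that runs lives, respawning and timed spawning of crates and pirates.
; BeginPlay shows the WG_Carga widget and starts a looping timer on the first GeneradorCubos.
; Tick triggers every GeneradorPiratas via timers whenever game time passes a threshold, which advances by an interval that shrinks toward a floor.
; REGENERARJUGADOR prints game over when no lives remain; otherwise it clears enemies and crates, decrements lives and possesses a new BP_Inti.
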(event `self.ReceiveBeginPlay`
  ;[1 1 1] PARAMETROS DE INICIO
  (`|ExecutionSequence`
    (:`then_0`
      (bind _returnvalue (`|CreateWidget` "/Game/Widget/WG_Carga.WG_Carga_C"))
      (`UserWidget.AddToViewport` _returnvalue 0))
    (:`then_1`
      (`self.spawncajas`))
    (:`then_2`
      (`KismetSystemLibrary.PrintString` (`KismetStringLibrary.Concat_StrStr` "VIDAS: " (`KismetStringLibrary.Conv_IntToString` (`self.VIDAS`)))))))

(event `self.ReceiveTick`
  (params (DeltaSeconds :type "Float (single-precision)"))
  ;[1 1 1] EVENTO TICK
  (`self.spawnpiratas`))

(event `spawncajas`
  ;[1 1 1] spawn cajas
  (bind _outactors (`GameplayStatics.GetAllActorsOfClass` "/Game/BpClass/GeneradorCubos.GeneradorCubos_C"))
  (bind _output_get (set `self.GeneradordeCajas` (`|GetArrayItem` _outactors)))
  (`KismetSystemLibrary.K2_SetTimer` _output_get "GENERADORDECAJAS" (`self.TimerSpawnCajas`) true))

(event `REGENERARJUGADOR`
  ;[1 1 1] REGENERAR PARTIDA SI JUGADOR TIENE VIDAS
  (if (`self.SINVIDAS`)
    ;;[1 1 1] GAME OVER
    (`KismetSystemLibrary.PrintString` "GAME OVER! ")
    (else
      ;;[1 1 1] destruir todos los enemigos al revivir
      (bind _outactors (`GameplayStatics.GetAllActorsOfClass` "/Game/Modelos/Enemigo/BP_Enemigos/enemigoCESAR.enemigoCESAR_C"))
      (for _array_element _outactors
        (`self.K2_DestroyActor` _array_element))
      ;;[1 1 1] destruir todas las cajas al revivir
      (bind _outactors_2 (`GameplayStatics.GetAllActorsOfClass` "/Game/BpClass/CAJA1.CAJA1_C"))
      (for _array_element_2 _outactors_2
        (`self.K2_DestroyActor` _array_element_2))
      (bind _outactors_3 (`GameplayStatics.GetAllActorsOfClass` "/Game/BpClass/CAJA1.CAJA1_C"))
      (for _array_element_3 _outactors_3
        (`self.K2_DestroyActor` _array_element_3))
      (bind _outactors_4 (`GameplayStatics.GetAllActorsOfClass` "/Game/BpClass/CAJA1.CAJA1_C"))
      (for _array_element_4 _outactors_4
        (`self.K2_DestroyActor` _array_element_4))
      (bind _result (`/Engine/EditorBlueprintResources/StandardMacros.DecrementInt` (`self.VIDAS`))
        (:`  `
          (if (not (> _result 1))
            (set `self.SINVIDAS` true))
          (`KismetSystemLibrary.PrintString` (`KismetStringLibrary.Concat_StrStr` "VIDAS: " (`KismetStringLibrary.Conv_IntToString` (`self.VIDAS`))))
          (bind _returnvalue (`|SpawnActorFromClass` "/Game/Modelos/Player/Blueprints/BP_Inti.BP_Inti_C" (`self.PUNTOGEGENERACION`) "Undefined" "OverrideRootScale" null null))
          (`Controller.Possess` (`GameplayStatics.GetPlayerController` 0) _returnvalue))))))

(event `spawnpiratas`
  (bind _ntimer (`self.NTimer`))
  (bind _limites (`self.limites`))
  ;[1 1 1] spawn PIRATAS
  (`/Engine/EditorBlueprintResources/StandardMacros.CompareFloat` (`KismetSystemLibrary.GetGameTimeInSeconds`) _limites
    (:`>`
      (if (not (== 2.0 _ntimer))
        (`/Engine/EditorBlueprintResources/StandardMacros.DecrementFloat` _ntimer
          (:`  `
            _)))
      (bind _output_get (set `self.limites` (+ _ntimer _limites)))
      (bind _outactors (`GameplayStatics.GetAllActorsOfClass` "/Game/BpClass/GeneradorPiratas.GeneradorPiratas_C"))
      (for _array_element _outactors
        (bind _output_get_2 (set `self.GeneradordePiratas` _array_element))
        (`KismetSystemLibrary.K2_SetTimer` _output_get_2 "GeneradordePiratas" 0.5)))))

(fn `UserConstructionScript`)