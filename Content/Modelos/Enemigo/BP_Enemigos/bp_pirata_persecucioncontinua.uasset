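; Pirate enemy Blueprint that patrols around its spawn point and chases and attacks the player (BP_Inti) on sight.
; Patrolling loops timed AI moves to randomized line-trace impact points within a patrol radius.
; Pawn sensing temporarily boosts walk speed and moves toward the player, playing one of two random attack montages on arrival.
; A retriggerable delay, refreshed by each sighting, calls patrol again once it expires.
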(event `self.ReceiveBeginPlay`
  ;[1 1 1] EVENTO BEGIN PLAY
  (set `self.puntopartida` (`self.K2_GetActorLocation`))
  (`self.Patrullar`))

(event `Patrullar`
  (bind (_puntopartida_x _puntopartida_y) (`KismetMathLibrary.BreakVector` (`self.puntopartida`)))
  (bind _returnvalue (+ (`KismetMathLibrary.RandomFloatInRange` (* -1 (`self.radioPatrulla`)) (`self.radioPatrulla`)) _puntopartida_x))
  (bind _returnvalue_2 (+ (`KismetMathLibrary.RandomFloatInRange` (* -1 (`self.radioPatrulla`)) (`self.radioPatrulla`)) _puntopartida_y))
  ;[1 1 1] Realiza un patrullaje en puntos ramdom.
  (bind _outhit (`KismetSystemLibrary.LineTraceSingle` (`KismetMathLibrary.MakeVector` _returnvalue _returnvalue_2 1500.0) (`KismetMathLibrary.MakeVector` _returnvalue _returnvalue_2) "TraceTypeQuery1" :!label _label))
  (`|AIMoveTo` self (`.ImpactPoint` (`GameplayStatics.BreakHitResult` _outhit)) null
    (:`then`
      (`KismetSystemLibrary.Delay` 3.0)
      (goto _label))))

(event `alcanzar`
  (params (velocidad :type "Float (double-precision)"))
  ;[1 1 1] Altera velocidad y despues de 10 segundos la disminuye
  (set `CharacterMovementComponent.MaxWalkSpeed` velocidad (`self.CharacterMovement`))
  (`KismetSystemLibrary.Delay` 10.0)
  (set `CharacterMovementComponent.MaxWalkSpeed` 300.0 (`self.CharacterMovement`)))

(event `self.PawnSensingEnemigo.OnSeePawn`
  (params (Pawn :type "Pawn Object Reference"))
  (bind _returnvalue (`AnimInstance.IsAnyMontagePlaying` (`SkeletalMeshComponent.GetAnimInstance` (`self.Mesh`))))
  ;[1 1 1] Detecta al player si el player esta en el rango de vision para seguirlo!
  (bind _asbp_inti (cast `/Game/Modelos/Player/Blueprints/BP_Inti` Pawn))
  (`self.alcanzar` 600.0)
  (if _returnvalue
    (`KismetSystemLibrary.RetriggerableDelay` 2.5 :!label _label_2)
    (`self.Patrullar`)
    (else
      (`|AIMoveTo` self (0.0 0.0 0.0) _asbp_inti 100.0
        (:`then`
          (goto _label_2))
        (:`OnSuccess`
          (if (not _returnvalue)
            (`|PlayMontage` (`self.Mesh`) (select `int` (`KismetMathLibrary.RandomIntegerInRange` 0 1) :`0` "/Game/Modelos/Enemigo/Animaciones/Am_Enemy_attack.Am_Enemy_attack" :`1` "/Game/Modelos/Enemigo/Animaciones/Am_Enemy_attack2.Am_Enemy_attack2" :!type "AnimMontage Object Reference"))))))))

(fn `UserConstructionScript`)