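; NPC Blueprint that wanders between waypoints and pauses to talk when the player approaches.
; Patrulla runs AIMoveTo toward one of three random waypoints, waits for Esperar seconds on success, then calls itself unless Hablando is set.
; The BoxConversa overlap sets Hablando only if the player enters while the NPC is standing; dialogue is just PrintString messages.
; End overlap clears Hablando but does not restart a stopped patrol.
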(event `self.ReceiveBeginPlay`
  (`self.Patrulla`))

(event `Patrulla`
  ;[1 1 1] Selecciona un target en un ramdon y se muve
  (if (not (`self.hablando`))
    (set `self.iswalk` true)
    (`|AIMoveTo` self (0.0 0.0 0.0) (`|GetArrayItem` (`|MakeArray` (`self.WayPoints1`) (`self.WayPoints2`) (`self.WayPoints3`)) (`KismetMathLibrary.RandomIntegerInRange` 0 2))
      (:`OnSuccess`
        (set `self.iswalk` false)
        (`KismetSystemLibrary.Delay` (`self.esperar`))
        (`self.Patrulla` self)))))

(event `self.BoxConversa.OnComponentBeginOverlap`
  (params (OverlappedComponent :type "PrimitiveComponent Object Reference") (OtherActor :type "Actor Object Reference") (OtherComp :type "PrimitiveComponent Object Reference") (OtherBodyIndex :type Integer) (bFromSweep :type Boolean) (SweepResult :type "HitResult Structure (by ref)"))
  ;[1 1 1] Detine al npc para conversar Conversacion
  (if (== (`GameplayStatics.GetPlayerPawn` 0) OtherActor)
    (if (`self.iswalk`)
      (`KismetSystemLibrary.PrintString` "Ahora no estoy ocupado")
      (else
        (`KismetSystemLibrary.PrintString` "Conversemos")
        (set `self.hablando` true)))))

(event `self.BoxConversa.OnComponentEndOverlap`
  (params (OverlappedComponent :type "PrimitiveComponent Object Reference") (OtherActor :type "Actor Object Reference") (OtherComp :type "PrimitiveComponent Object Reference") (OtherBodyIndex :type Integer))
  ;[1 1 1] Detine al npc para conversar Conversacion
  (`KismetSystemLibrary.PrintString` "Chau!!")
  (set `self.hablando` false))

(fn `UserConstructionScript`)