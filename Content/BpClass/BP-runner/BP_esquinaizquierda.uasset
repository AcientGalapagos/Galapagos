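; BP_esquinaizquierda is a left-corner piece for the runner that reacts when the player (BP_Inti) overlaps its trigger boxes.
; All three boxes set PuedeGirar on BP_Inti to true, allowing it to turn.
; Box1 and Box2 also apply Danyo damage through REDUCIRVIDA before enabling the turn.
; The construction script only calls its parent.
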(event `self.Box.OnComponentBeginOverlap`
  (params (OverlappedComponent :type "PrimitiveComponent Object Reference") (OtherActor :type "Actor Object Reference") (OtherComp :type "PrimitiveComponent Object Reference") (OtherBodyIndex :type Integer) (bFromSweep :type Boolean) (SweepResult :type "HitResult Structure (by ref)"))
  (bind _asbp_inti (cast `/Game/Personajes/Player/Blueprints/BP_Inti` OtherActor))
  (set `/Game/Personajes/Player/Blueprints/BP_Inti.PuedeGirar` true _asbp_inti))

(event `self.Box1.OnComponentBeginOverlap`
  (params (OverlappedComponent :type "PrimitiveComponent Object Reference") (OtherActor :type "Actor Object Reference") (OtherComp :type "PrimitiveComponent Object Reference") (OtherBodyIndex :type Integer) (bFromSweep :type Boolean) (SweepResult :type "HitResult Structure (by ref)"))
  (bind _asbp_inti (cast `/Game/Personajes/Player/Blueprints/BP_Inti` OtherActor))
  (`/Game/Personajes/Player/Blueprints/BP_Inti.REDUCIRVIDA` _asbp_inti (`self.danyo`))
  (set `/Game/Personajes/Player/Blueprints/BP_Inti.PuedeGirar` true _asbp_inti))

(event `self.Box2.OnComponentBeginOverlap`
  (params (OverlappedComponent :type "PrimitiveComponent Object Reference") (OtherActor :type "Actor Object Reference") (OtherComp :type "PrimitiveComponent Object Reference") (OtherBodyIndex :type Integer) (bFromSweep :type Boolean) (SweepResult :type "HitResult Structure (by ref)"))
  (bind _asbp_inti (cast `/Game/Personajes/Player/Blueprints/BP_Inti` OtherActor))
  (`/Game/Personajes/Player/Blueprints/BP_Inti.REDUCIRVIDA` _asbp_inti (`self.danyo`))
  (set `/Game/Personajes/Player/Blueprints/BP_Inti.PuedeGirar` true _asbp_inti))

(fn `UserConstructionScript`
  (`parent.UserConstructionScript`))