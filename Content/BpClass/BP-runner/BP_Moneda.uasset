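; BP_Moneda is a collectible coin for a runner game that awards points to the BP_Inti player.
; A timeline started on BeginPlay drives the coin's vertical offset, and Tick spins it by a fixed, frame-dependent step.
; When BP_Inti overlaps the box, the coin plays a sound at the player, calls SUMAPUNTOS, raises the local score and fruit counter, then destroys itself.
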(event `self.ReceiveBeginPlay`
  ;[1 1 1] Movimiento Constante Moneda
  (bind (_direction _movimiento) (`Timeline|MoverMoneda`)
    (:`Update`
      (`SceneComponent.K2_SetRelativeLocation` (`self.Moneda`) (`KismetMathLibrary.MakeVector` 0.0 0.0 _movimiento) false false))))

(event `self.ReceiveTick`
  (params (DeltaSeconds :type "Float (single-precision)"))
  ;[1 1 1] Movimiento Constante Moneda
  (`SceneComponent.K2_AddRelativeRotation` (`self.Moneda`) (struct :`Yaw` 1.5) false false))

(event `self.Box.OnComponentBeginOverlap`
  (params (OverlappedComponent :type "PrimitiveComponent Object Reference") (OtherActor :type "Actor Object Reference") (OtherComp :type "PrimitiveComponent Object Reference") (OtherBodyIndex :type Integer) (bFromSweep :type Boolean) (SweepResult :type "HitResult Structure (by ref)"))
  ;[1 1 1] Colisión Moneda-Player
  (bind _asbp_inti (cast `/Game/Personajes/Player/Blueprints/BP_Inti` OtherActor))
  (`GameplayStatics.PlaySoundAtLocation` "/Engine/VREditor/Sounds/UI/Teleport_Mode_Entered.Teleport_Mode_Entered" (`self.K2_GetActorLocation` _asbp_inti) (struct) 1.0 1.0 0.0 null null null)
  (`/Game/Personajes/Player/Blueprints/BP_Inti.SUMAPUNTOS` _asbp_inti 1.0)
  (set `/Game/Personajes/Player/Blueprints/BP_Inti.PuntuacionLocal` (+ (`/Game/Personajes/Player/Blueprints/BP_Inti.PuntuacionLocal` _asbp_inti) 100) _asbp_inti)
  (bind _result (`/Engine/EditorBlueprintResources/StandardMacros.IncrementInt` (`/Game/Personajes/Player/Blueprints/BP_Inti.contadorfrutas` _asbp_inti))
    (:`  `
      (set `/Game/Personajes/Player/Blueprints/BP_Inti.contadorfrutas` _result _asbp_inti)
      (`self.K2_DestroyActor`))))

(fn `UserConstructionScript`)