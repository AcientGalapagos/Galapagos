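; Runner platform actor, apparently a parent class, that populates itself with randomly placed coins and a map actor on BeginPlay.
; When CrearObstaculo is set, it reveals one of eight obstacles; a timeline slides the movable one.
; Obstacles cost BP_Inti a life and trigger death; PIEDRA breaks the destructibles and door, which hurt Inti on end overlap instead.
; Inti leaving the Box destroys the platform after a delay.
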(event `self.ReceiveBeginPlay`
  (bind _obstaculo_7_movible (`self.Obstaculo 7 Movible`))
  ;[1 1 1] Inicio
  (`|ExecutionSequence`
    (:`then_0`
      ;[1 1 1] SpawnMonedas
      (for _ (range 1 (+ (`KismetMathLibrary.RandomIntegerInRange` 1 3) 1))
        (bind _returnvalue (`|SpawnActorFromClass` "/Game/BpClass/BP-runner/BP_Moneda.BP_Moneda_C" (`KismetMathLibrary.MakeTransform` (+ (`KismetMathLibrary.GreaterGreater_VectorRotator` (`KismetMathLibrary.MakeVector` (`KismetMathLibrary.RandomFloatInRange` 100.0 1500.0) (`KismetMathLibrary.RandomFloatInRange` -600.0 600.0) (`KismetMathLibrary.RandomFloatInRange` 70.0 80.0)) (`self.K2_GetActorRotation`)) (`self.K2_GetActorLocation`))) "Undefined" "OverrideRootScale" null null))
        (`KismetArrayLibrary.Array_Add` (`self.Monedas`) _returnvalue)))
    (:`then_1`
      ;[1 1 1] SpawnObstaculos
      (if (`self.CrearObstaculo`)
        (bind _output_get (set `self.ObstaculoSeleccionar` (select `int` (`KismetMathLibrary.RandomIntegerInRange` 0 7) :`0` (`self.Obstaculo1`) :`1` (`self.Obstaculo2`) :`2` (`self.Obstaculo3`) :`3` (`self.Obstaculo4 Saltable`) :`4` (`self.Obstaculo5 Destructible`) :`5` (`self.Obstaculo6 Destructible2`) :`6` (`self.Obstaculo 7 Movible`) :`7` (`self.Obstaculo 8 Puerta`))))
        (`SceneComponent.SetVisibility` _output_get true false)
        (`PrimitiveComponent.SetCollisionProfileName` _output_get "OverlapAll" true)
        ;[1 1 1] MuroMóvil
        (if (== _output_get (`self.Obstaculo 7 Movible`))
          (`KismetArrayLibrary.Array_Add` (`self.MurosMoviles`)))))
    (:`then_2`
      (bind (_direction _movimiento) (`Timeline|MovimientoPlataforma`)
        (:`Update`
          (`/Engine/EditorBlueprintResources/StandardMacros.IsValid` _obstaculo_7_movible
            (:`Is Valid`
              (`SceneComponent.K2_SetRelativeLocation` _obstaculo_7_movible (`KismetMathLibrary.MakeVector` 0.0 _movimiento) false false)
              ;[1 1 1] DestruccionMovilesCada2Segundos
              (for _array_element (`self.MurosMoviles`)
                (`/Engine/EditorBlueprintResources/StandardMacros.IsValid` _array_element
                  (:`Is Valid`
                    (`self.K2_DestroyActor`)))))))))
    (:`then_3`
      ;[1 1 1] Spawn Puzzle
      (for _ (range 1 (+ (`KismetMathLibrary.RandomIntegerInRange` 1 1) 1))
        (bind _returnvalue_2 (`|SpawnActorFromClass` "/Game/BpClass/BP-runner/BP_MapaRunner.BP_MapaRunner_C" (`KismetMathLibrary.MakeTransform` (+ (`KismetMathLibrary.GreaterGreater_VectorRotator` (`KismetMathLibrary.MakeVector` (`KismetMathLibrary.RandomFloatInRange` 100.0 1500.0) (`KismetMathLibrary.RandomFloatInRange` -600.0 600.0) (`KismetMathLibrary.RandomFloatInRange` 75.0 80.0)) (`self.K2_GetActorRotation`)) (`self.K2_GetActorLocation`))) "Undefined" "OverrideRootScale" null null))
        (`KismetArrayLibrary.Array_Add` (`self.Mapa`) _returnvalue_2)))))

(event `self.Box.OnComponentEndOverlap`
  (params (OverlappedComponent :type "PrimitiveComponent Object Reference") (OtherActor :type "Actor Object Reference") (OtherComp :type "PrimitiveComponent Object Reference") (OtherBodyIndex :type Integer))
  ;[1 1 1] DestruccionPlataformasCada2Segundos
  (cast `/Game/Personajes/Player/Blueprints/BP_Inti` OtherActor)
  (`KismetSystemLibrary.Delay` 2.0)
  (`self.K2_DestroyActor`)
  ;[1 1 1] DestruccionMonedasCada2Segundos
  (for _array_element (`self.Monedas`)
    (`/Engine/EditorBlueprintResources/StandardMacros.IsValid` _array_element
      (:`Is Valid`
        (`self.K2_DestroyActor`)))))

(event `self.ReceiveHit`
  (params (MyComp :type "PrimitiveComponent Object Reference") (Other :type "Actor Object Reference") (OtherComp :type "PrimitiveComponent Object Reference") (bSelfMoved :type Boolean) (HitLocation :type "Vector Structure") (HitNormal :type "Vector Structure") (NormalImpulse :type "Vector Structure") (Hit :type "HitResult Structure (by ref)"))
  ;[1 1 1] ParículasAlMomentoDeSaltar
  (cast `/Game/Personajes/Player/Blueprints/BP_Inti` Other)
  (`GameplayStatics.SpawnEmitterAtLocation` "/Engine/Tutorial/SubEditors/TutorialAssets/TutorialParticleSystem.TutorialParticleSystem" HitLocation))

(event `self.Obstaculo1.OnComponentBeginOverlap`
  (params (OverlappedComponent :type "PrimitiveComponent Object Reference") (OtherActor :type "Actor Object Reference") (OtherComp :type "PrimitiveComponent Object Reference") (OtherBodyIndex :type Integer) (bFromSweep :type Boolean) (SweepResult :type "HitResult Structure (by ref)"))
  ;[1 1 1] EventosAlMomentoDeColisionarYMorir
  (bind _asbp_inti (cast `/Game/Personajes/Player/Blueprints/BP_Inti` OtherActor))
  (`/Game/Personajes/Player/Blueprints/BP_Inti.RestarVidas` _asbp_inti)
  (`/Game/Personajes/Player/Blueprints/BP_Inti.EventoMorir` _asbp_inti)
  (`GameplayStatics.PlaySoundAtLocation` "/Engine/EditorSounds/GamePreview/PossessPlayer.PossessPlayer" (`self.K2_GetActorLocation` _asbp_inti) (struct) 1.5 1.0 0.0 null null null)
  (`ActorComponent.K2_DestroyComponent` OverlappedComponent))

(event `self.Obstaculo2.OnComponentBeginOverlap`
  (params (OverlappedComponent :type "PrimitiveComponent Object Reference") (OtherActor :type "Actor Object Reference") (OtherComp :type "PrimitiveComponent Object Reference") (OtherBodyIndex :type Integer) (bFromSweep :type Boolean) (SweepResult :type "HitResult Structure (by ref)"))
  ;[1 1 1] EventosAlMomentoDeColisionarYMorir
  (bind _asbp_inti (cast `/Game/Personajes/Player/Blueprints/BP_Inti` OtherActor))
  (`/Game/Personajes/Player/Blueprints/BP_Inti.RestarVidas` _asbp_inti)
  (`/Game/Personajes/Player/Blueprints/BP_Inti.EventoMorir` _asbp_inti)
  (`GameplayStatics.PlaySoundAtLocation` "/Engine/EditorSounds/GamePreview/PossessPlayer.PossessPlayer" (`self.K2_GetActorLocation` _asbp_inti) (struct) 1.5 1.0 0.0 null null null)
  (`ActorComponent.K2_DestroyComponent` OverlappedComponent))

(event `self.Obstaculo5 Destructible.OnComponentBeginOverlap`
  (params (OverlappedComponent :type "PrimitiveComponent Object Reference") (OtherActor :type "Actor Object Reference") (OtherComp :type "PrimitiveComponent Object Reference") (OtherBodyIndex :type Integer) (bFromSweep :type Boolean) (SweepResult :type "HitResult Structure (by ref)"))
  ;[1 1 1] Bloques destructibles
  (bind _aspiedra (cast `/Game/BpClass/PIEDRA` OtherActor))
  (`GameplayStatics.PlaySoundAtLocation` "/Engine/VREditor/Sounds/UI/Laser_Push.Laser_Push" (`self.K2_GetActorLocation` _aspiedra) (struct) 2.0 1.0 0.0 null null null)
  (`ActorComponent.K2_DestroyComponent` OverlappedComponent)
  (`self.K2_DestroyActor` _aspiedra))

(event `self.Obstaculo3.OnComponentBeginOverlap`
  (params (OverlappedComponent :type "PrimitiveComponent Object Reference") (OtherActor :type "Actor Object Reference") (OtherComp :type "PrimitiveComponent Object Reference") (OtherBodyIndex :type Integer) (bFromSweep :type Boolean) (SweepResult :type "HitResult Structure (by ref)"))
  ;[1 1 1] EventosAlMomentoDeColisionarYMorir
  (bind _asbp_inti (cast `/Game/Personajes/Player/Blueprints/BP_Inti` OtherActor))
  (`/Game/Personajes/Player/Blueprints/BP_Inti.RestarVidas` _asbp_inti)
  (`/Game/Personajes/Player/Blueprints/BP_Inti.EventoMorir` _asbp_inti)
  (`GameplayStatics.PlaySoundAtLocation` "/Engine/EditorSounds/GamePreview/PossessPlayer.PossessPlayer" (`self.K2_GetActorLocation` _asbp_inti) (struct) 1.5 1.0 0.0 null null null)
  (`ActorComponent.K2_DestroyComponent` OverlappedComponent))

(event `self.Obstaculo6 Destructible2.OnComponentBeginOverlap`
  (params (OverlappedComponent :type "PrimitiveComponent Object Reference") (OtherActor :type "Actor Object Reference") (OtherComp :type "PrimitiveComponent Object Reference") (OtherBodyIndex :type Integer) (bFromSweep :type Boolean) (SweepResult :type "HitResult Structure (by ref)"))
  ;[1 1 1] Bloques destructibles
  (bind _aspiedra (cast `/Game/BpClass/PIEDRA` OtherActor))
  (`GameplayStatics.PlaySoundAtLocation` "/Engine/VREditor/Sounds/UI/Laser_Push.Laser_Push" (`self.K2_GetActorLocation` _aspiedra) (struct) 2.0 1.0 0.0 null null null)
  (`ActorComponent.K2_DestroyComponent` OverlappedComponent)
  (`self.K2_DestroyActor` _aspiedra))

(event `self.Obstaculo4 Saltable.OnComponentBeginOverlap`
  (params (OverlappedComponent :type "PrimitiveComponent Object Reference") (OtherActor :type "Actor Object Reference") (OtherComp :type "PrimitiveComponent Object Reference") (OtherBodyIndex :type Integer) (bFromSweep :type Boolean) (SweepResult :type "HitResult Structure (by ref)"))
  ;[1 1 1] EventosAlMomentoDeColisionarYMorir
  (bind _asbp_inti (cast `/Game/Personajes/Player/Blueprints/BP_Inti` OtherActor))
  (`/Game/Personajes/Player/Blueprints/BP_Inti.RestarVidas` _asbp_inti)
  (`/Game/Personajes/Player/Blueprints/BP_Inti.EventoMorir` _asbp_inti)
  (`GameplayStatics.PlaySoundAtLocation` "/Engine/EditorSounds/GamePreview/PossessPlayer.PossessPlayer" (`self.K2_GetActorLocation` _asbp_inti) (struct) 1.5 1.0 0.0 null null null)
  (`ActorComponent.K2_DestroyComponent` OverlappedComponent))

(event `self.Obstaculo 7 Movible.OnComponentBeginOverlap`
  (params (OverlappedComponent :type "PrimitiveComponent Object Reference") (OtherActor :type "Actor Object Reference") (OtherComp :type "PrimitiveComponent Object Reference") (OtherBodyIndex :type Integer) (bFromSweep :type Boolean) (SweepResult :type "HitResult Structure (by ref)"))
  ;[1 1 1] EventosAlMomentoDeColisionarYMorir
  (bind _asbp_inti (cast `/Game/Personajes/Player/Blueprints/BP_Inti` OtherActor))
  (`/Game/Personajes/Player/Blueprints/BP_Inti.RestarVidas` _asbp_inti)
  (`/Game/Personajes/Player/Blueprints/BP_Inti.EventoMorir` _asbp_inti)
  (`GameplayStatics.PlaySoundAtLocation` "/Engine/EditorSounds/GamePreview/PossessPlayer.PossessPlayer" (`self.K2_GetActorLocation` _asbp_inti) (struct) 1.5 1.0 0.0 null null null)
  (`ActorComponent.K2_DestroyComponent` OverlappedComponent))

(event `self.Obstaculo 8 Puerta.OnComponentBeginOverlap`
  (params (OverlappedComponent :type "PrimitiveComponent Object Reference") (OtherActor :type "Actor Object Reference") (OtherComp :type "PrimitiveComponent Object Reference") (OtherBodyIndex :type Integer) (bFromSweep :type Boolean) (SweepResult :type "HitResult Structure (by ref)"))
  ;[1 1 1] AbrirPuertaConPiedra
  (bind _aspiedra (cast `/Game/BpClass/PIEDRA` OtherActor))
  (`GameplayStatics.PlaySoundAtLocation` "/Engine/VREditor/Sounds/UI/Laser_Push.Laser_Push" (`self.K2_GetActorLocation` _aspiedra) (struct) 2.0 1.0 0.0 null null null)
  (`ActorComponent.K2_DestroyComponent` OverlappedComponent)
  (`self.K2_DestroyActor` _aspiedra))

(event `self.Obstaculo5 Destructible.OnComponentEndOverlap`
  (params (OverlappedComponent :type "PrimitiveComponent Object Reference") (OtherActor :type "Actor Object Reference") (OtherComp :type "PrimitiveComponent Object Reference") (OtherBodyIndex :type Integer))
  ;[1 1 1] EventosAlMomentoDeColisionarYMorir
  (bind _asbp_inti (cast `/Game/Personajes/Player/Blueprints/BP_Inti` OtherActor))
  (`/Game/Personajes/Player/Blueprints/BP_Inti.RestarVidas` _asbp_inti)
  (`/Game/Personajes/Player/Blueprints/BP_Inti.EventoMorir` _asbp_inti)
  (`GameplayStatics.PlaySoundAtLocation` "/Engine/EditorSounds/GamePreview/PossessPlayer.PossessPlayer" (`self.K2_GetActorLocation` _asbp_inti) (struct) 1.5 1.0 0.0 null null null)
  (`ActorComponent.K2_DestroyComponent` OverlappedComponent))

(event `self.Obstaculo6 Destructible2.OnComponentEndOverlap`
  (params (OverlappedComponent :type "PrimitiveComponent Object Reference") (OtherActor :type "Actor Object Reference") (OtherComp :type "PrimitiveComponent Object Reference") (OtherBodyIndex :type Integer))
  ;[1 1 1] EventosAlMomentoDeColisionarYMorir
  (bind _asbp_inti (cast `/Game/Personajes/Player/Blueprints/BP_Inti` OtherActor))
  (`/Game/Personajes/Player/Blueprints/BP_Inti.RestarVidas` _asbp_inti)
  (`/Game/Personajes/Player/Blueprints/BP_Inti.EventoMorir` _asbp_inti)
  (`GameplayStatics.PlaySoundAtLocation` "/Engine/EditorSounds/GamePreview/PossessPlayer.PossessPlayer" (`self.K2_GetActorLocation` _asbp_inti) (struct) 1.5 1.0 0.0 null null null)
  (`ActorComponent.K2_DestroyComponent` OverlappedComponent))

(event `self.Obstaculo 8 Puerta.OnComponentEndOverlap`
  (params (OverlappedComponent :type "PrimitiveComponent Object Reference") (OtherActor :type "Actor Object Reference") (OtherComp :type "PrimitiveComponent Object Reference") (OtherBodyIndex :type Integer))
  ;[1 1 1] EventosAlMomentoDeColisionarYMorir
  (bind _asbp_inti (cast `/Game/Personajes/Player/Blueprints/BP_Inti` OtherActor))
  (`/Game/Personajes/Player/Blueprints/BP_Inti.RestarVidas` _asbp_inti)
  (`/Game/Personajes/Player/Blueprints/BP_Inti.EventoMorir` _asbp_inti)
  (`GameplayStatics.PlaySoundAtLocation` "/Engine/EditorSounds/GamePreview/PossessPlayer.PossessPlayer" (`self.K2_GetActorLocation` _asbp_inti) (struct) 1.5 1.0 0.0 null null null)
  (`ActorComponent.K2_DestroyComponent` OverlappedComponent))

(fn `UserConstructionScript`)