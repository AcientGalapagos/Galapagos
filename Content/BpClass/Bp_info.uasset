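; Bp_info is an info sign trigger that gives the player a message while they stand inside its box.
; When the player pawn begins overlapping BoxLetrero, it copies its Mensaje value as text into the Mensaje variable on the BP_Inti character.
; When the player leaves the box, it clears that variable.
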(event `self.BoxLetrero.OnComponentBeginOverlap`
  (params (OverlappedComponent :type "PrimitiveComponent Object Reference") (OtherActor :type "Actor Object Reference") (OtherComp :type "PrimitiveComponent Object Reference") (OtherBodyIndex :type Integer) (bFromSweep :type Boolean) (SweepResult :type "HitResult Structure (by ref)"))
  (if (== (`GameplayStatics.GetPlayerPawn` 0) OtherActor)
    (bind _asbp_inti (cast `/Game/Personajes/Player/Blueprints/BP_Inti` (`GameplayStatics.GetPlayerCharacter` 0)))
    (set `/Game/Personajes/Player/Blueprints/BP_Inti.Mensaje` (`KismetTextLibrary.Conv_StringToText` (`self.Mensaje`)) _asbp_inti)))

(event `self.BoxLetrero.OnComponentEndOverlap`
  (params (OverlappedComponent :type "PrimitiveComponent Object Reference") (OtherActor :type "Actor Object Reference") (OtherComp :type "PrimitiveComponent Object Reference") (OtherBodyIndex :type Integer))
  (if (== (`GameplayStatics.GetPlayerPawn` 0) OtherActor)
    (bind _asbp_inti (cast `/Game/Personajes/Player/Blueprints/BP_Inti` (`GameplayStatics.GetPlayerCharacter` 0)))
    (set `/Game/Personajes/Player/Blueprints/BP_Inti.Mensaje` "" _asbp_inti)))

(fn `UserConstructionScript`)