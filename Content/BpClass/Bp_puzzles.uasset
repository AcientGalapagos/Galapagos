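; Puzzle Blueprint where the player must step on four buttons in a fixed order (3, 1, 2, 4) to unlock progress toward the final challenge.
; Box overlaps by the player advance a shared counter, turning the correct button to the OK material with a click sound.
; A wrong step flashes all buttons bad, plays an error and resets.
; Completion locks the puzzle and sets the Puzzles flag on BP_Inti.
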(event `self.Box1.OnComponentBeginOverlap`
  (params (OverlappedComponent :type "PrimitiveComponent Object Reference") (OtherActor :type "Actor Object Reference") (OtherComp :type "PrimitiveComponent Object Reference") (OtherBodyIndex :type Integer) (bFromSweep :type Boolean) (SweepResult :type "HitResult Structure (by ref)"))
  ;[1 1 1] Valida la secuencia en que se tiene que pulsar las botones
  (if (`self.resuelto`)
    _
    (elif (== OtherActor (`GameplayStatics.GetPlayerPawn` 0))
      (set `self.conclics` (+ (`self.conclics`) 1))
      (if (== (`self.conclics`) 2)
        (`PrimitiveComponent.SetMaterial` (`self.btn1`) 0 "/Game/Materiales/MatOk.MatOk")
        (`GameplayStatics.PlaySoundAtLocation` "/Game/Audios/clicbtn.clicbtn" (0.0 0.0 0.0) (struct) 1.0 1.0 0.0 null null null :!label _label)
        (if (== (`self.conclics`) 4)
          (set `self.resuelto` true)
          (set `/Game/Modelos/Player/Blueprints/BP_Inti.puzzles` true (cast `/Game/Modelos/Player/Blueprints/BP_Inti` (`GameplayStatics.GetPlayerPawn` 0) :!pure true))
          (`KismetSystemLibrary.PrintString` "Perfecto!! ve hacia la puerta tu reto final te aguarda!"))
        (else
          (`self.puzzerror`))))))

(event `self.Box2.OnComponentBeginOverlap`
  (params (OverlappedComponent :type "PrimitiveComponent Object Reference") (OtherActor :type "Actor Object Reference") (OtherComp :type "PrimitiveComponent Object Reference") (OtherBodyIndex :type Integer) (bFromSweep :type Boolean) (SweepResult :type "HitResult Structure (by ref)"))
  ;[1 1 1] Valida la secuencia en que se tiene que pulsar las botones
  (if (`self.resuelto`)
    _
    (elif (== (`GameplayStatics.GetPlayerPawn` 0) OtherActor)
      (set `self.conclics` (+ (`self.conclics`) 1))
      (if (== (`self.conclics`) 3)
        (`PrimitiveComponent.SetMaterial` (`self.btn2`) 0 "/Game/Materiales/MatOk.MatOk")
        (goto _label)
        (else
          (`self.puzzerror`))))))

(event `self.Box3.OnComponentBeginOverlap`
  (params (OverlappedComponent :type "PrimitiveComponent Object Reference") (OtherActor :type "Actor Object Reference") (OtherComp :type "PrimitiveComponent Object Reference") (OtherBodyIndex :type Integer) (bFromSweep :type Boolean) (SweepResult :type "HitResult Structure (by ref)"))
  ;[1 1 1] Valida la secuencia en que se tiene que pulsar las botones
  (if (`self.resuelto`)
    _
    (elif (== (`GameplayStatics.GetPlayerPawn` 0) OtherActor)
      (set `self.conclics` (+ (`self.conclics`) 1))
      (if (== (`self.conclics`) 1)
        (`PrimitiveComponent.SetMaterial` (`self.btn3`) 0 "/Game/Materiales/MatOk.MatOk")
        (goto _label)
        (else
          (`self.puzzerror`))))))

(event `self.Box4.OnComponentBeginOverlap`
  (params (OverlappedComponent :type "PrimitiveComponent Object Reference") (OtherActor :type "Actor Object Reference") (OtherComp :type "PrimitiveComponent Object Reference") (OtherBodyIndex :type Integer) (bFromSweep :type Boolean) (SweepResult :type "HitResult Structure (by ref)"))
  ;[1 1 1] Valida la secuencia en que se tiene que pulsar las botones
  (if (`self.resuelto`)
    _
    (elif (== (`GameplayStatics.GetPlayerPawn` 0) OtherActor)
      (set `self.conclics` (+ (`self.conclics`) 1))
      (if (== (`self.conclics`) 4)
        (`PrimitiveComponent.SetMaterial` (`self.btn4`) 0 "/Game/Materiales/MatOk.MatOk")
        (goto _label)
        (else
          (`self.puzzerror`))))))

(event `puzzerror`
  ;[1 1 1] Funcion error
  (`PrimitiveComponent.SetMaterial` (`self.btn3`) 0 "/Game/Materiales/MatBad.MatBad")
  (`PrimitiveComponent.SetMaterial` (`self.btn1`) 0 "/Game/Materiales/MatBad.MatBad")
  (`PrimitiveComponent.SetMaterial` (`self.btn2`) 0 "/Game/Materiales/MatBad.MatBad")
  (`PrimitiveComponent.SetMaterial` (`self.btn4`) 0 "/Game/Materiales/MatBad.MatBad")
  (set `self.conclics` 0)
  (`GameplayStatics.PlaySoundAtLocation` "/Game/Audios/error.error" (0.0 0.0 0.0) (struct) 1.0 1.0 0.0 null null null)
  (`KismetSystemLibrary.Delay` 1.0)
  (`PrimitiveComponent.SetMaterial` (`self.btn3`) 0 "/Game/Materiales/MatYellow.MatYellow")
  (`PrimitiveComponent.SetMaterial` (`self.btn1`) 0 "/Game/Materiales/MatYellow.MatYellow")
  (`PrimitiveComponent.SetMaterial` (`self.btn2`) 0 "/Game/Materiales/MatYellow.MatYellow")
  (`PrimitiveComponent.SetMaterial` (`self.btn4`) 0 "/Game/Materiales/MatYellow.MatYellow"))

(event `ConsultaResuelto`
  (`KismetSystemLibrary.PrintString` "Pasa" (`self.resuelto`)))

(fn `UserConstructionScript`)