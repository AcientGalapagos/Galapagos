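; Sea lion rescue zone that, when a CAJAFOCAS crate hits it, destroys the crate and adds to BP_Inti's sea lion counter and score.
; The first and second rescues show a message, teleport the player and advance the game mode phase; the first also spawns a crate and enemy and swaps tagged phase actors.
; Later hits reveal FINRESCATE actors once combined animal rescues total fifteen, otherwise destroy FASE2 actors.
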(event `self.ReceiveHit`
  (params (MyComp :type "PrimitiveComponent Object Reference") (Other :type "Actor Object Reference") (OtherComp :type "PrimitiveComponent Object Reference") (bSelfMoved :type Boolean) (HitLocation :type "Vector Structure") (HitNormal :type "Vector Structure") (NormalImpulse :type "Vector Structure") (Hit :type "HitResult Structure (by ref)"))
  (bind _returnvalue (`GameplayStatics.GetPlayerPawn` 0))
  (bind _charactermovement (`Character.CharacterMovement` (cast `/Game/Personajes/Player/Blueprints/BP_Inti` _returnvalue :!pure true)))
  ;[1 1 1] incrementa contador de leones marinos
  (bind _ascajafocas (cast `/Game/BpClass/CAJAFOCAS` Other))
  (`self.K2_DestroyActor` _ascajafocas)
  (bind _asbp_inti (cast `/Game/Personajes/Player/Blueprints/BP_Inti` (`GameplayStatics.GetPlayerCharacter` 0)))
  (`/Game/Personajes/Player/Blueprints/BP_Inti.IncContadorLeones` _asbp_inti)
  (`/Game/Personajes/Player/Blueprints/BP_Inti.SUMAPUNTOS` _asbp_inti (`self.puntos`))
  (if (== (`/Game/Personajes/Player/Blueprints/BP_Inti.LEONESRESCATADOS` _asbp_inti) 1.0)
    (set `/Game/Personajes/Player/Blueprints/BP_Inti.Mensaje` (`self.MSGFASE1`) _asbp_inti)
    (`CharacterMovementComponent.DisableMovement` _charactermovement)
    (`KismetSystemLibrary.Delay` 4.0)
    (set `/Game/Personajes/Player/Blueprints/BP_Inti.Mensaje` "" _asbp_inti)
    (`Controller.Possess` (`GameplayStatics.GetPlayerController` 0) _returnvalue)
    (`self.K2_TeleportTo` _asbp_inti (`self.posicionplayermision1`) (struct :`Yaw` 35.0))
    (bind _asbp_gm_tercera_persona (cast `/Game/BpClass/BP_GM_terceraPersona` (`GameplayStatics.GetGameMode`)))
    (`/Game/BpClass/BP_GM_terceraPersona.NIVELYCUENTA` _asbp_gm_tercera_persona (`self.fase2`))
    (`|SpawnActorFromClass` "/Game/BpClass/CAJAFOCAS.CAJAFOCAS_C" (`self.posicioncaja1`) "Undefined" "OverrideRootScale" null null)
    (`|SpawnActorFromClass` "/Game/Personajes/Enemigo/BP_Enemigos/Bp_Enemigo.Bp_Enemigo_C" (`self.posicionENEMIGO`) "Undefined" "OverrideRootScale" null null)
    (bind _outactors (`GameplayStatics.GetAllActorsWithTag` "FASE1"))
    (for _array_element _outactors
      (`self.SetActorHiddenInGame` _array_element true)
      (`self.K2_DestroyActor` _array_element))
    (bind _outactors_2 (`GameplayStatics.GetAllActorsWithTag` "FASE2"))
    (for _array_element_2 _outactors_2
      (`self.SetActorHiddenInGame` _array_element_2 false))
    (elif (== (`/Game/Personajes/Player/Blueprints/BP_Inti.LEONESRESCATADOS` _asbp_inti) 2.0)
      (set `/Game/Personajes/Player/Blueprints/BP_Inti.Mensaje` (`self.MSGFASE2`) _asbp_inti)
      (`CharacterMovementComponent.DisableMovement` _charactermovement)
      (`KismetSystemLibrary.Delay` 4.0)
      (set `/Game/Personajes/Player/Blueprints/BP_Inti.Mensaje` "" _asbp_inti)
      (`Controller.Possess` (`GameplayStatics.GetPlayerController` 0) _returnvalue)
      (`self.K2_TeleportTo` _asbp_inti (`self.posicionplayermision1`) (struct :`Yaw` 35.0))
      (bind _asbp_gm_tercera_persona_2 (cast `/Game/BpClass/BP_GM_terceraPersona` (`GameplayStatics.GetGameMode`)))
      (`/Game/BpClass/BP_GM_terceraPersona.NIVELYCUENTA` _asbp_gm_tercera_persona_2 (`self.fase3`))
      (else
        ;[1 1 1] incrementa contador iguanas
        (if (== (+ (`/Game/Personajes/Player/Blueprints/BP_Inti.LEONESRESCATADOS` _asbp_inti) (`/Game/Personajes/Player/Blueprints/BP_Inti.TORTUGASRESCATADAS` _asbp_inti) (`/Game/Personajes/Player/Blueprints/BP_Inti.IGUANASRESCATADAS` _asbp_inti)) 15.0)
          (set `/Game/Personajes/Player/Blueprints/BP_Inti.Mensaje` (`self.MSGFIN`) _asbp_inti)
          (`KismetSystemLibrary.Delay` 4.0)
          (set `/Game/Personajes/Player/Blueprints/BP_Inti.Mensaje` (`self.MSGMOCHILA`) _asbp_inti)
          (`KismetSystemLibrary.Delay` 4.0)
          (set `/Game/Personajes/Player/Blueprints/BP_Inti.Mensaje` "" _asbp_inti)
          (bind _outactors_3 (`GameplayStatics.GetAllActorsWithTag` "FINRESCATE"))
          (for _array_element_3 _outactors_3
            (`self.SetActorHiddenInGame` _array_element_3 false))
          (else
            (bind _outactors_4 (`GameplayStatics.GetAllActorsWithTag` "FASE2"))
            (for _array_element_4 _outactors_4
              (`self.SetActorHiddenInGame` _array_element_4 true)
              (`self.K2_DestroyActor` _array_element_4))))))))

(fn `UserConstructionScript`)