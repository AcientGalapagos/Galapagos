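; Enemy wave spawner that creates groups of Bp_Enemigo at three placed points and starts each one patrolling.
; GeneraOleada computes the enemy total and loops over waves, calling GenerarEnemigos immediately for the first and through a Delay for later ones.
; That Delay sits inside the loop, so it does not space successive waves apart.
; GenerarEnemigos re-rolls the random point after each spawn to avoid consecutive repeats.
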(event `GeneraOleada`
  (`KismetSystemLibrary.PrintString` "Oleada 1" true true (struct :`R` 0.557292 :`G` 0.121783 :`B` 0.066218 :`A` 1.0) 10.0)
  (set `self.TotalEnemigos` (* (`self.TotalOleadas`) (`self.EnemigosXOleada`)))
  (for _index (range 1 (+ (`self.TotalOleadas`) 1))
    (if (== _index 1)
      (`self.GenerarEnemigos`)
      (else
        (`KismetSystemLibrary.Delay` (`self.IntervaloSpanw`))
        (`self.GenerarEnemigos`)))))

(event `GenerarEnemigos`
  (bind _output_get (set `self.Lastspan` (`KismetMathLibrary.RandomIntegerInRange` 0 2)))
  (for _ (range 1 (+ (`self.EnemigosXOleada`) 1))
    (bind _returnvalue (`|SpawnActorFromClass` "/Game/Personajes/Enemigo/BP_Enemigos/Bp_Enemigo.Bp_Enemigo_C" (`KismetMathLibrary.MakeTransform` (`self.K2_GetActorLocation` (`|GetArrayItem` (`|MakeArray` (`self.Punto1`) (`self.Punto2`) (`self.Punto3`)) _output_get)) (struct :`Yaw` -150.0)) "Undefined" "OverrideRootScale" null null))
    (`/Game/Personajes/Enemigo/BP_Enemigos/Bp_Enemigo.Patrullar` _returnvalue)
    (for _ (range 11)
      (bind _output_get_2 (set `self.NewSpan` (`KismetMathLibrary.RandomIntegerInRange` 0 2)))
      (if (!= _output_get_2 (`self.Lastspan`))
        (set `self.Lastspan` (`self.NewSpan`))
        (break)))))

(fn `UserConstructionScript`)