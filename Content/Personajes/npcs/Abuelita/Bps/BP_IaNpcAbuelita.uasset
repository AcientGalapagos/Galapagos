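; Grandmother NPC Blueprint that wanders between waypoints and gives the player dialogue about pirates taking the island's species.
; Patrulla loops by moving to one of three random waypoints with AIMoveTo, waiting, then repeating unless Hablando is set.
; BoxConversa overlap shows a brush-off through BP_Inti's PrintMensaje while walking, otherwise sets Hablando and delivers the quest plea.
; End overlap clears Hablando and says goodbye, but does not restart Patrulla.
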(event `self.ReceiveBeginPlay`
  (`self.Patrulla`))

(event `Patrulla`
  ;[1 1 1] Selecciona un target en un ramdon y se muve
  (if (not (`self.hablando`))
    (set `self.iswalk` true)
    (`|AIMoveTo` self (0.0 0.0 0.0) (`|GetArrayItem` (`|MakeArray` (`self.WayPoints1`) (`self.WayPoints2`) (`self.WayPoints3`)) (`KismetMathLibrary.RandomIntegerInRange` 0 2))
      (:`OnSuccess`
        (set `self.iswalk` false)
        (`KismetSystemLibrary.Delay` (`self.esperar`))
        (`self.Patrulla` self)))))

(event `self.BoxConversa.OnComponentBeginOverlap`
  (params (OverlappedComponent :type "PrimitiveComponent Object Reference") (OtherActor :type "Actor Object Reference") (OtherComp :type "PrimitiveComponent Object Reference") (OtherBodyIndex :type Integer) (bFromSweep :type Boolean) (SweepResult :type "HitResult Structure (by ref)"))
  ;[1 1 1] Detine al npc para conversar Conversacion
  (if (== (`GameplayStatics.GetPlayerPawn` 0) OtherActor)
    (if (`self.iswalk`)
      (bind _asbp_inti (cast `/Game/Personajes/Player/Blueprints/BP_Inti` (`GameplayStatics.GetPlayerCharacter` 0)))
      (`/Game/Personajes/Player/Blueprints/BP_Inti.PrintMensaje` _asbp_inti "Ahora no estoy preocupada." 5.0)
      (else
        (set `self.hablando` true)
        (bind _asbp_inti_2 (cast `/Game/Personajes/Player/Blueprints/BP_Inti` (`GameplayStatics.GetPlayerCharacter` 0)))
        (`/Game/Personajes/Player/Blueprints/BP_Inti.PrintMensaje` _asbp_inti_2 "Algo terrible ha pasado, Hay piratas en la isla y se estan llevando las especies. Por favor encuentralas a todas." 15.0)))))

(event `self.BoxConversa.OnComponentEndOverlap`
  (params (OverlappedComponent :type "PrimitiveComponent Object Reference") (OtherActor :type "Actor Object Reference") (OtherComp :type "PrimitiveComponent Object Reference") (OtherBodyIndex :type Integer))
  ;[1 1 1] Detine al npc para conversar Conversacion
  (set `self.hablando` false)
  (bind _asbp_inti (cast `/Game/Personajes/Player/Blueprints/BP_Inti` (`GameplayStatics.GetPlayerCharacter` 0)))
  (`/Game/Personajes/Player/Blueprints/BP_Inti.PrintMensaje` _asbp_inti "Hasta pronto" 3.0))

(fn `UserConstructionScript`)