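; Enemy character that patrols, chases and attacks the player (BP_Inti).
; It walks to random line-traced points around its spawn; pawn sensing triggers a temporary speed boost and chase, with a random attack montage on arrival.
; Damage is separate from the montages: a looping timer hits the player while overlapping.
; At zero health it increments the player's kill count, plays a death montage, destroys itself and decrements the GameMode's active rescue pirate count.
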(event `RESETVARIABLES`
  ;[1 1 1] RESET VARIABLES
  (`|ExecutionSequence`
    (:`then_0`
      (set `self.ESTASVIVO` true)
      (set `self.puedemoverse` true))
    (:`then_1`
      (set `self.VIDA` 100))))

(event `REDUCIRVIDA`
  (params (`DAÑO` :type Integer))
  ;[1 1 1] reducir vida en un ataque
  (if (`self.ESTASVIVO`)
    (bind _output_get (set `self.VIDA` (- (`self.VIDA`) `DAÑO`)))
    (if (<= _output_get 0)
      (set `self.ESTASVIVO` false)
      (set `self.puedemoverse` false)
      (bind _asbp_inti (cast `/Game/Personajes/Player/Blueprints/BP_Inti` (`GameplayStatics.GetPlayerCharacter` 0)))
      (set `/Game/Personajes/Player/Blueprints/BP_Inti.ENEMIGOSMUERTOS` (+ (`/Game/Personajes/Player/Blueprints/BP_Inti.ENEMIGOSMUERTOS` _asbp_inti) 1.0) _asbp_inti)
      (`|PlayMontage` (`self.Mesh`) "/Game/Personajes/Enemigo/Animaciones/Montg_Muerte.Montg_Muerte"
        (:`then`
          (`KismetSystemLibrary.Delay` 2.0)
          (`self.K2_DestroyActor`)
          (bind _asbp_gm_tercera_persona (cast `/Game/BpClass/BP_GM_terceraPersona` (`GameplayStatics.GetGameMode`)))
          (bind _result (`/Engine/EditorBlueprintResources/StandardMacros.DecrementInt` (`/Game/BpClass/BP_GM_terceraPersona.PIRATASACTIVORESCATE` _asbp_gm_tercera_persona))
            (:`  `
              (bind _output_get_2 (set `/Game/BpClass/BP_GM_terceraPersona.PIRATASACTIVORESCATE` _result _asbp_gm_tercera_persona))
              (`KismetSystemLibrary.PrintString` (`KismetStringLibrary.Conv_IntToString` _output_get_2))))))
      (else
        (set `self.ESTASVIVO` true)))))

(event `self.ReceiveBeginPlay`
  ;[1 1 1] EVENTO BEGIN PLAY
  (`|ExecutionSequence`
    (:`then_0`
      (set `self.puntopartida` (`self.K2_GetActorLocation`))
      (`self.Patrullar`))
    (:`then_1`
      (`self.RESETVARIABLES`))))

(event `Patrullar`
  (bind (_puntopartida_x _puntopartida_y) (`KismetMathLibrary.BreakVector` (`self.puntopartida`)))
  (bind _returnvalue (+ (`KismetMathLibrary.RandomFloatInRange` (* -1 (`self.radioPatrulla`)) (`self.radioPatrulla`)) _puntopartida_x))
  (bind _returnvalue_2 (+ (`KismetMathLibrary.RandomFloatInRange` (* -1 (`self.radioPatrulla`)) (`self.radioPatrulla`)) _puntopartida_y))
  ;[1 1 1] Realiza un patrullaje en puntos ramdom.
  (if (`self.puedemoverse`)
    (bind _outhit (`KismetSystemLibrary.LineTraceSingle` (`KismetMathLibrary.MakeVector` _returnvalue _returnvalue_2 3000.0) (`KismetMathLibrary.MakeVector` _returnvalue _returnvalue_2) "TraceTypeQuery1" :!label _label))
    (`|AIMoveTo` self (`.ImpactPoint` (`GameplayStatics.BreakHitResult` _outhit)) null
      (:`then`
        (`KismetSystemLibrary.Delay` 5.0)
        (goto _label)))))

(event `alcanzar`
  (params (velocidad :type "Float (double-precision)"))
  ;[1 1 1] Altera velocidad y despues de 10 segundos la disminuye
  (if (`self.puedemoverse`)
    (set `CharacterMovementComponent.MaxWalkSpeed` velocidad (`self.CharacterMovement`))
    (`KismetSystemLibrary.Delay` 30.0)
    (set `CharacterMovementComponent.MaxWalkSpeed` 300.0 (`self.CharacterMovement`))))

(event `self.PawnSensingEnemigo.OnSeePawn`
  (params (Pawn :type "Pawn Object Reference"))
  (bind _returnvalue (`AnimInstance.IsAnyMontagePlaying` (`SkeletalMeshComponent.GetAnimInstance` (`self.Mesh`))))
  ;[1 1 1] Detecta al player si el player esta en el rango de vision para seguirlo!
  (bind _asbp_inti (cast `/Game/Personajes/Player/Blueprints/BP_Inti` Pawn))
  (`self.alcanzar` 600.0)
  (if _returnvalue
    (`KismetSystemLibrary.RetriggerableDelay` 2.5 :!label _label_2)
    (`self.Patrullar`)
    (else
      (`|AIMoveTo` self (0.0 0.0 0.0) _asbp_inti 500.0
        (:`then`
          (goto _label_2))
        (:`OnSuccess`
          (if (not _returnvalue)
            (set `self.puedemoverse` false)
            (`|PlayMontage` (`self.Mesh`) (select `int` (`KismetMathLibrary.RandomIntegerInRange` 0 1) :`0` "/Game/Personajes/Enemigo/Animaciones/Am_Enemy_attack.Am_Enemy_attack" :`1` "/Game/Personajes/Enemigo/Animaciones/Am_Enemy_attack2.Am_Enemy_attack2" :!type "AnimMontage Object Reference")
              (:`OnCompleted`
                (set `self.puedemoverse` true)))))))))

(event `self.ReceiveActorBeginOverlap`
  (params (OtherActor :type "Actor Object Reference"))
  ;[1 1 1] ATAQUE A PERSONAJE PRINCIPAL
  (bind _asbp_inti (cast `/Game/Personajes/Player/Blueprints/BP_Inti` OtherActor))
  (bind _output_get (set `self.JugadorImpactado` _asbp_inti))
  (bind _returnvalue (`KismetSystemLibrary.K2_SetTimerDelegate` (delegate `ATACAR`) (`self.tiempoacaque`) true)))

(event `ATACAR`
  ;[1 1 1] ATAQUE A PERSONAJE PRINCIPAL
  (`/Game/Personajes/Player/Blueprints/BP_Inti.IMPACTO` (stale `self.ReceiveActorBeginOverlap` _output_get) (`self.DAÑO`)))

(event `self.ReceiveActorEndOverlap`
  (params (OtherActor :type "Actor Object Reference"))
  ;[1 1 1] ATAQUE A PERSONAJE PRINCIPAL
  (if (== OtherActor (`self.JugadorImpactado`))
    (`KismetSystemLibrary.K2_ClearAndInvalidateTimerHandle` (stale `self.ReceiveActorBeginOverlap` _returnvalue))))

(fn `UserConstructionScript`)